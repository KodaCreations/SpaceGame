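; Star actor that shows its owner (neutral or either player) through its flare sprite and highlights on cursor hover or selection.
; A color-matched flipbook plays on hover, then repeats from frame 15 to skip the zoom-in.
; Losing hover while unselected, or selection of another actor, runs a timeline that scales the flipbook out, preserving rotation.
; A Reverse flag lets a new hover interrupt the zoom-out by snapping back to normal size.
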(event OnFinishedPlaying(Animation)
  (bind _animation (Variables|Default|GetAnimation))
  ;[1 1 1] When finished animation, playback from after zoom (frame 15)
  (Class|PaperFlipbookComponent|SetPlaybackPositioninFrames _animation 15 false)
  (Audio|Components|Audio|Play _animation))

(event Custom|Selection%20is%20made
  (params (Newly%20selected%20actor :type Star%20Blueprint%20Object%20Reference))
  ;[1 1 1] When a new selection is made and new selected actor is not this
  (if (not (== Newly%20selected%20actor self))
    ;[1 1 1] Zoom out by scaling animation flip book (in order to keep the rotation)
    (Variables|Default|SetReverse true)
    (bind _track (Timeline|ZoomOutTimeline PlayFromStart)
      (:Update
        ;;[1 1 1] Stop scaling if reverse becomes false
        (if (Variables|Default|GetReverse)
          (Transformation|SetWorldScale3D (Variables|Default|GetAnimation) (+ (* "1.000000, 0,1.000000" _track) "0,1.000000, 0"))))
      (:Finished
        (Variables|Default|SetReverse false)))))

(event EventBeginPlay
  (bind _animation (Variables|Default|GetAnimation))
  (bind _sprite (Variables|Default|GetSprite))
  ;[1 1 1] Set animation and to not loop
  (switch Utilities|FlowControl|Switch|SwitchonStarColor (Variables|Default|Getcolor)
    (:Red
      (Sprite|SetFlipbook _animation "/Game/GUI/flipStarRed.flipStarRed"))
    (:Yellow
      (Sprite|SetFlipbook _animation "/Game/GUI/flipStarYellow.flipStarYellow"))
    (:Blue
      (Sprite|SetFlipbook _animation "/Game/GUI/flipStarBlue.flipStarBlue"))
    (:Orange
      (Sprite|SetFlipbook _animation "/Game/GUI/flipStarOrange.flipStarOrange")))
  (Audio|Components|Audio|Stop _animation)
  (Components|Timeline|SetLooping _animation false)
  ;[1 1 1] Switch sprite color on start
  (switch Utilities|FlowControl|Switch|SwitchonOwnedBy (Variables|Default|GetownedBy)
    (:Neutral
      (Rendering|Components|Sprite|SetSprite _sprite "/Game/Assets/Textures/StarSprites/starFlareGray_Sprite.starFlareGray_Sprite"))
    (:Player1
      (Rendering|Components|Sprite|SetSprite _sprite "/Game/Assets/Textures/StarSprites/starFlareGreen_Sprite.starFlareGreen_Sprite"))
    (:Player2
      (Rendering|Components|Sprite|SetSprite _sprite "/Game/Assets/Textures/StarSprites/starFlareRed_Sprite.starFlareRed_Sprite"))))

(event MouseInput|EventActorBeginCursorOver
  (bind _animation (Variables|Default|GetAnimation))
  ;[1 1 1] On curser over and not already selected, branch on reverse bool
  (bind _asmouse_pawn (Utilities|Casting|CastToMousePawn (Pawn|GetControlledPawn (Game|GetPlayerController 0))))
  (bind _returnvalue (Class|MousePawn|GetSelectedActor _asmouse_pawn))
  (if (not (== _returnvalue self))
    (Variables|Default|SetMouseIsOver true)
    (if (Variables|Default|GetReverse)
      ;[1 1 1] If reversing, zoom back to normal size (instant looks just as good as timeline zoom)
      (Variables|Default|SetReverse false)
      (Transformation|SetWorldScale3D _animation "0.500000,1.000000,0.500000")
      (else
        ;[1 1 1] If not reversing, play animation from beginning
        (Transformation|SetWorldScale3D _animation "0.500000,1.000000,0.500000")
        (Components|Timeline|PlayfromStart _animation)
        (Rendering|SetVisibility _animation true false)))))

(event EventOwnerChanged
  (bind _sprite (Variables|Default|GetSprite))
  ;[1 1 1] When owner changes, change sprite
  (switch Utilities|FlowControl|Switch|SwitchonOwnedBy (Variables|Default|GetownedBy)
    (:Neutral
      (Rendering|Components|Sprite|SetSprite _sprite "/Game/Assets/Textures/StarSprites/starFlareGray_Sprite.starFlareGray_Sprite"))
    (:Player1
      (Rendering|Components|Sprite|SetSprite _sprite "/Game/Assets/Textures/StarSprites/starFlareGreen_Sprite.starFlareGreen_Sprite"))
    (:Player2
      (Rendering|Components|Sprite|SetSprite _sprite "/Game/Assets/Textures/StarSprites/starFlareRed_Sprite.starFlareRed_Sprite"))))

(event MouseInput|EventActorEndCursorOver
  ;[1 1 1] MouseOver ends and actor is not selected
  (bind _asmouse_pawn (Utilities|Casting|CastToMousePawn (Pawn|GetControlledPawn (Game|GetPlayerController 0))))
  (bind _returnvalue (Class|MousePawn|GetSelectedActor _asmouse_pawn))
  (if (not (== _returnvalue self))
    ;[1 1 1] Zoom out by scaling animation flip book (in order to keep the rotation)
    (Variables|Default|SetReverse true)
    (bind _track (Timeline|ZoomOutTimeline PlayFromStart)
      (:Update
        ;;[1 1 1] Stop scaling if reverse becomes false
        (if (Variables|Default|GetReverse)
          (Transformation|SetWorldScale3D (Variables|Default|GetAnimation) (+ (* "1.000000, 0,1.000000" _track) "0,1.000000, 0"))))
      (:Finished
        (Variables|Default|SetReverse false)))))

(fn ConstructionScript)