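; Behavior Tree task that makes the enemy AI send a fleet from its selected star to its target star.
; It reads the Selected and Target stars from the Blackboard and passes them to SendFleetTo on the EnemyAIController.
; After sending, it resets both keys to NullStar.
; The task finishes as successful even when a cast fails and no fleet is sent.
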(event EventReceiveExecute
  (params (OwnerActor :type Actor%20Object%20Reference))
  (bind _nullstar (Variables|Default|GetNullStar))
  ;[1 1 1] Send Fleet
  (bind _asenemy_aicontroller (Utilities|Casting|CastToEnemyAIController OwnerActor)
    (:then
      (bind _asstar (Utilities|Casting|CastToStar (Class|BTFunctionLibrary|GetBlackboardValueasObject (Variables|Default|GetSelected)))
        (:then
          (bind _asstar_2 (Utilities|Casting|CastToStar (Class|BTFunctionLibrary|GetBlackboardValueasObject (Variables|Default|GetTarget)))
            (:then
              (Class|EnemyAIController|SendFleetto _asenemy_aicontroller _asstar _asstar_2)
              ;[1 1 1] Reset Target and Selected
              (Class|BTFunctionLibrary|SetBlackboardValueasObject (Variables|Default|GetSelected) _nullstar)
              (Class|BTFunctionLibrary|SetBlackboardValueasObject (Variables|Default|GetTarget) _nullstar))
            (:CastFailed
              _)))
        (:CastFailed
          _)))
    (:CastFailed
      _))
  (AI|BehaviorTree|FinishExecute true))