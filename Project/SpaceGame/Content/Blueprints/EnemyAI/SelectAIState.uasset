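; Behavior tree node that scores an enemy's stars on tick to select its AI state on the blackboard.
; It resets the EnemyAIController's values, then sums and prints CalculateValueOfStar over each star.
; The sign check on the total is unfinished: both outcomes write the first EnemyAIState to the State key, and the setters for the other two states are unconnected.
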(event EventTick
  (params (OwnerActor :type Actor%20Object%20Reference) (DeltaSeconds :type Float%20%28single-precision%29))
  (Variables|Default|SetAIValue 0.0)
  ;[1 1 1] Calculate Star Values
  (bind _asenemy_aicontroller (Utilities|Casting|CastToEnemyAIController OwnerActor))
  (Class|EnemyAIController|ResetValues _asenemy_aicontroller)
  (bind _returnvalue (Class|EnemyAIController|GetStars _asenemy_aicontroller))
  (for (_array_element _array_index) _returnvalue
    (bind _returnvalue_2 (Class|EnemyAIController|CalculateValueOfStar _asenemy_aicontroller _array_element _array_index))
    (Variables|Default|SetAIValue (+ (Variables|Default|GetAIValue) _returnvalue_2)))
  (Development|PrintText (Utilities|Text|ToText(Float) (Variables|Default|GetAIValue) "HalfToEven"))
  ;[1 1 1] Calculate AI State
  (if (< (stale _output_get) 0.0)
    _
    (else
      _))
  (Class|BTFunctionLibrary|SetBlackboardValueasEnum (Variables|Default|GetState) (Utilities|Enum|LiteralenumEnemyAIState "NewEnumerator0")))