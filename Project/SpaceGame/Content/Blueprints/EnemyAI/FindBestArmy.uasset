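; Behavior tree task that chooses which enemy AI stars to move ships between, based on fleet size.
; Around the blackboard Target star, it picks the Player2-owned star with the largest fleet as the destination.
; A top-two scan of all the AI's stars picks the second-largest fleet as the source.
; It overwrites Target with the destination, stores the source in Selected, and reports success even if casts fail.
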(event EventTick
  (params (OwnerActor :type Actor%20Object%20Reference) (DeltaSeconds :type Float%20%28single-precision%29))
  (Variables|Default|SetHighestNrOfShips 0.0)
  (Variables|Default|SetMostShipsByTarget 0.0)
  (Variables|Default|SetSecoundNrOfShips 0.0)
  (bind _asenemy_aicontroller (Utilities|Casting|CastToEnemyAIController OwnerActor)
    (:then
      (bind _asstar (Utilities|Casting|CastToStar (Class|BTFunctionLibrary|GetBlackboardValueasObject (Variables|Default|GetTarget)))
        (:then
          (bind _returnvalue (Class|EnemyAIController|GetSurroundingStarsat _asenemy_aicontroller _asstar))
          (for _array_element _returnvalue
            (if (Utilities|Enum|Equal(Enum) (Variables|/Script/SpaceGame.Star|GetownedBy _array_element) (Utilities|Enum|LiteralenumOwnedBy "Player2"))
              ;[1 1 1] Set  Star To Move To
              (bind _returnvalue_2 (Class|Star|GetFleet _array_element))
              (if (!= _returnvalue_2 0)
                (bind _returnvalue_3 (Class|Fleet|GetSize _returnvalue_2))
                (if (> _returnvalue_3 (Variables|Default|GetMostShipsByTarget))
                  (Variables|Default|SetMoveTo _array_element)
                  (Variables|Default|SetMostShipsByTarget _returnvalue_3)))))
          (bind _returnvalue_4 (Class|EnemyAIController|GetMyStars _asenemy_aicontroller))
          (for _array_element_2 _returnvalue_4
            (bind _returnvalue_5 (Class|Star|GetFleet _array_element_2))
            (if (!= _returnvalue_5 0)
              ;[1 1 1] Set  Star To Move From
              (bind _returnvalue_6 (Class|Fleet|GetSize _returnvalue_5))
              (if (> _returnvalue_6 (Variables|Default|GetHighestNrOfShips))
                (Variables|Default|SetMoveFrom (Variables|Default|GetHighestValueStar))
                (Variables|Default|SetSecoundNrOfShips (Variables|Default|GetHighestNrOfShips))
                (Variables|Default|SetHighestValueStar _array_element_2)
                (Variables|Default|SetHighestNrOfShips _returnvalue_6)
                (elif (> _returnvalue_6 (Variables|Default|GetSecoundNrOfShips))
                  (Variables|Default|SetMoveFrom _array_element_2)
                  (Variables|Default|SetSecoundNrOfShips _returnvalue_6)))))
          ;[1 1 1] Set MoveTo and MoveFrom
          (Class|BTFunctionLibrary|SetBlackboardValueasObject (Variables|Default|GetTarget) (Variables|Default|GetMoveTo))
          (Class|BTFunctionLibrary|SetBlackboardValueasObject (Variables|Default|GetSelected) (Variables|Default|GetMoveFrom))
          (AI|BehaviorTree|FinishExecute true))
        (:CastFailed
          (AI|BehaviorTree|FinishExecute true :!label _label))))
    (:CastFailed
      (goto _label))))