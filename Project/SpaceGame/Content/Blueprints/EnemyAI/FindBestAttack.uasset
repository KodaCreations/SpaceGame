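; Behavior tree tick logic for the enemy AI that picks which star to attack and which fleet to send.
; It scores surrounding stars through the EnemyAIController and finds the owned star holding the largest fleet.
; Player1 targets get one attack state if that fleet exceeds a size threshold and another otherwise, while other targets always get the first.
; When a target exists, it writes AttackState, Selected (fleet's star) and Target to the Blackboard.
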(event EventTick
  (params (OwnerActor :type Actor%20Object%20Reference) (DeltaSeconds :type Float%20%28single-precision%29))
  (bind _asenemy_aicontroller (Utilities|Casting|CastToEnemyAIController OwnerActor))
  ;[1 1 1] Find Best Star To Attack
  (Variables|Default|SetBestAttackValue -1e+03)
  (Variables|Default|SetBestStarValueWithFleet -1e+03)
  (bind _returnvalue (Class|EnemyAIController|GetSurroundingStars _asenemy_aicontroller))
  (for _array_element _returnvalue
    (bind _returnvalue_2 (Class|EnemyAIController|GetValueOfStar _asenemy_aicontroller _array_element))
    (if (> _returnvalue_2 (Variables|Default|GetBestAttackValue))
      (Variables|Default|SetBestStarToAttack _array_element)
      (Variables|Default|SetBestAttackValue _returnvalue_2)))
  ;[1 1 1] Find Best Fleet To Attack With
  (bind _returnvalue_3 (Class|EnemyAIController|GetMyStars _asenemy_aicontroller))
  (for _array_element_2 _returnvalue_3
    (bind _returnvalue_4 (Class|Star|GetFleet _array_element_2))
    (if (!= _returnvalue_4 0)
      (bind _returnvalue_5 (Class|Fleet|GetSize _returnvalue_4))
      (if (> _returnvalue_5 (Variables|Default|GetBestStarValueWithFleet))
        (Variables|Default|SetBestStarWithFleet _array_element_2)
        (Variables|Default|SetBestStarValueWithFleet _returnvalue_5))))
  ;[1 1 1] Check If Worth Attacking Enemy
  (if (!= (Variables|Default|GetBestStarToAttack) 0)
    (if (Utilities|Enum|Equal(Enum) (Variables|/Script/SpaceGame.Star|GetownedBy (Variables|Default|GetBestStarToAttack)) "Player1")
      (if (> (Variables|Default|GetBestStarValueWithFleet) 1e+01)
        ;[1 1 1] Set Attack State
        (Class|BTFunctionLibrary|SetBlackboardValueasEnum (Variables|Default|GetAttackState) (Utilities|Enum|LiteralenumEnemyAttackState "NewEnumerator0") :!label _label)
        (else
          (Class|BTFunctionLibrary|SetBlackboardValueasEnum (Variables|Default|GetAttackState) (Utilities|Enum|LiteralenumEnemyAttackState "NewEnumerator1"))))
      (else
        (goto _label)))
    ;[1 1 1] Set Selected and Target
    (Class|BTFunctionLibrary|SetBlackboardValueasObject (Variables|Default|GetSelected) (Variables|Default|GetBestStarWithFleet))
    (Class|BTFunctionLibrary|SetBlackboardValueasObject (Variables|Default|GetTarget) (Variables|Default|GetBestStarToAttack))))