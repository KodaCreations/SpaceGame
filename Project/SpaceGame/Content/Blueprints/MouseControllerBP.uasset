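; MouseControllerBP is a player controller that turns mouse clicks on stars into commands for the controlled MousePawn.
; Releasing either button line-traces under the cursor on the Visibility channel and casts the hit actor to Star.
; Left click selects the hit star on the pawn, or deselects when no star is hit.
; Right click on a star tells the pawn to send a fleet to it.
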(event EventBeginPlay)

(event EventTick
  (params (DeltaSeconds :type Float%20%28single-precision%29)))

(event Input|MouseEvents|RightMouseButton
  (params (Key :type Key%20Structure :default "AnyKey"))
  (:Released
    (bind _asstar (Utilities|Casting|CastToStar (.HitActor (Collision|BreakHitResult (.HitResult (Game|Player|GetHitResultUnderCursorbyChannel "TraceTypeQuery1" true))))))
    (bind _asmouse_pawn (Utilities|Casting|CastToMousePawn (Pawn|GetControlledPawn)))
    (Class|MousePawn|SendFleetto _asmouse_pawn _asstar)))

(event Input|MouseEvents|LeftMouseButton
  (params (Key :type Key%20Structure :default "AnyKey"))
  (:Released
    (bind _asstar (Utilities|Casting|CastToStar (.HitActor (Collision|BreakHitResult (.HitResult (Game|Player|GetHitResultUnderCursorbyChannel "TraceTypeQuery1" true)))))
      (:then
        (bind _asmouse_pawn (Utilities|Casting|CastToMousePawn (Pawn|GetControlledPawn)))
        (Class|MousePawn|SelectStar _asmouse_pawn _asstar))
      (:CastFailed
        (bind _asmouse_pawn_2 (Utilities|Casting|CastToMousePawn (Pawn|GetControlledPawn)))
        (Class|MousePawn|Deselect _asmouse_pawn_2)))))

(fn ConstructionScript)