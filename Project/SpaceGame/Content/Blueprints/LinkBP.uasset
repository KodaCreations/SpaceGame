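; LinkBP is an actor that draws a straight sprite link between two referenced actors, Star1 and Star2.
; Its construction script moves the actor to the midpoint of the two stars.
; It then aligns the sprite's pitch and yaw with the direction between them and scales its length by their distance, keeping it thin.
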(fn ConstructionScript
  (bind _sprite (Variables|Default|GetSprite))
  (bind _star1 (Variables|Default|GetStar1))
  (bind _star2 (Variables|Default|GetStar2))
  (bind _returnvalue (Transformation|GetActorLocation _star2))
  (bind _returnvalue_2 (Transformation|GetActorLocation _star1))
  (bind _returnvalue_3 (- _returnvalue_2 _returnvalue))
  (bind _returnvalue_4 (Math|Vector|Normalize _returnvalue_3))
  (bind _returnvalue_5 (Math|Conversions|RotationFromXVector _returnvalue_4))
  (bind (_roll _pitch _yaw) (Math|Rotator|BreakRotator _returnvalue_5))
  (Transformation|SetActorLocation (/ (+ (Transformation|GetActorLocation _star1) (Transformation|GetActorLocation _star2)) 2) false false)
  (Transformation|SetRelativeRotation _sprite (Math|Rotator|MakeRotator 0.0 _pitch _yaw) false false)
  (Transformation|SetRelativeScale3D _sprite (Math|Vector|MakeVector (/ (Math|Vector|VectorLength (- (Transformation|GetActorLocation _star1) (Transformation|GetActorLocation _star2))) 4e+02) 1.0 0.1)))